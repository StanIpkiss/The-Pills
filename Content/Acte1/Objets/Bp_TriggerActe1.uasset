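; Trigger volume in Act 1 that moves the game on to Act 2.
; On BeginPlay it caches the Gm_GameModeThePills game mode.
; When the player character overlaps the box while BpLily's Conversation flag is true, it sets that flag true again, calls InteragirAvecCible on the game mode with itself, then opens the Acte2 level.
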(event `self.ReceiveBeginPlay`
  (bind _asgm_game_mode_the_pills (cast `/Game/System/Gm_GameModeThePills` (`GameplayStatics.GetGameMode`)))
  (set `self.As Gm Game Mode The Pills` _asgm_game_mode_the_pills))

(event `self.Box.OnComponentBeginOverlap`
  (params (OverlappedComponent :type "PrimitiveComponent Object Reference") (OtherActor :type "Actor Object Reference") (OtherComp :type "PrimitiveComponent Object Reference") (OtherBodyIndex :type Integer) (bFromSweep :type Boolean) (SweepResult :type "HitResult Structure (by ref)"))
  (bind _bp_lily (`self.Bp_Lily`))
  ;[1 1 1] Passage a l'acte 2
  (if (and (== OtherActor (`GameplayStatics.GetPlayerCharacter` 0)) (`/Game/Lily/Bp_Lily.Conversation` _bp_lily))
    (set `/Game/Lily/Bp_Lily.Conversation` true _bp_lily)
    (`/Game/System/Gm_GameModeThePills.InteragirAvecCible` (`self.As Gm Game Mode The Pills`) self)
    (`GameplayStatics.OpenLevel` "Acte2")))

(fn `UserConstructionScript`)