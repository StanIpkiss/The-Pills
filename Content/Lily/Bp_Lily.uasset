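; Lily is an interactable character Blueprint that shows her dialogue one line per interaction.
; On Interagir it calls TalkDialogue, then notifies the Gm_GameModeThePills game mode cached at BeginPlay through InteragirAvecCible.
; TalkDialogue increments TalkIndex and displays that Dialogue entry in a lazily created Ui_Dialogue widget.
; Once the index passes the last entry, it removes the widget from its parent without resetting the index.
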(event `self.ReceiveBeginPlay`
  (bind _asgm_game_mode_the_pills (cast `/Game/System/Gm_GameModeThePills` (`GameplayStatics.GetGameMode`)))
  (set `self.As Gm Game Mode The Pills` _asgm_game_mode_the_pills))

(event `/Game/Dialogue/Bp_Interagir.Interagir`
  (set `self.Conversation` true)
  (if (`self.Conversation`)
    (`self.TalkDialogue`)
    (`/Game/System/Gm_GameModeThePills.InteragirAvecCible` (`self.As Gm Game Mode The Pills`) self)))

(fn `TalkDialogue`
  (`/Engine/EditorBlueprintResources/StandardMacros.IncrementInt` (`self.TalkIndex`)
    (:`  `
      (if (< (`self.TalkIndex`) (`KismetArrayLibrary.Array_Length` (`self.Dialogue`)))
        (`self.DialogueUIRef`
          (:`then`
            _)
          (:`else`
            (bind _returnvalue (`|CreateWidget` "/Game/Dialogue/Ui/Ui_Dialogue.Ui_Dialogue_C" (`GameplayStatics.GetPlayerController` 0)))
            (set `self.DialogueUIRef` _returnvalue)
            (`UserWidget.AddToViewport` _returnvalue 0)))
        (`TextBlock.SetText` (`/Game/Dialogue/Ui/Ui_Dialogue.TalkText` (`self.DialogueUIRef`)) (`KismetTextLibrary.Conv_StringToText` (`|GetArrayItem` (`self.Dialogue`) (`self.TalkIndex`))))
        (else
          (`Widget.RemoveFromParent` (`self.DialogueUIRef`)))))))

(fn `UserConstructionScript`)