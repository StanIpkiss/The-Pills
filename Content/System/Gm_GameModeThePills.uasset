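; Game mode that runs a linear mission chain and shows the current mission's text on screen.
; On BeginPlay it creates the UI_Missions widget and displays the mission marked EnCours from the Missions struct array.
; InteragirAvecCible takes an interacted actor and, if it is an active mission's target, marks that mission Terminée, activates the next array entry and refreshes the widget.
; After the last mission the text is left unchanged.
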(event `self.ReceiveBeginPlay`
  (bind _returnvalue (`|CreateWidget` "/Game/UI/UI_Missions.UI_Missions_C" (`GameplayStatics.GetPlayerController` 0)))
  (set `self.UiMissionRef` _returnvalue)
  (`UserWidget.AddToViewport` _returnvalue 0)
  (`self.AfficherMissionEncoursUI`))

(fn `AfficherMissionEncoursUI`
  (for _array_element (`self.Missions`)
    (bind (_mission _description _etat) (break `/Game/Structure/S_Missions` _array_element))
    (switch `/Game/Structure/Enum_EtatMission` _etat
      (:`NewEnumerator1`
        (`TextBlock.SetText` (`/Game/UI/UI_Missions.TextMission` (`self.UiMissionRef`)) (`KismetTextLibrary.Conv_StringToText` _mission))))))

(fn `InteragirAvecCible`
  (params (Actor :type "Actor Object Reference"))
  (locals (IndexRef :type Integer) (MissionRef :type "/Game/Structure/S_Missions Structure") (NextIndex :type Integer))
  ;[1 1 1] Cherche si l'acteur avec qui on interagis correspond a la mission en cours
  (for (_array_element _array_index) (`self.Missions`)
    (set `self.Array Index` _array_index)
    (set `self.Array Element` _array_element)
    (bind (_mission _description _etat _cible) (break `/Game/Structure/S_Missions` _array_element))
    (if (and (`|EnumEquality` _etat "NewEnumerator1") (== _cible Actor))
      ;[1 1 1] Mission Terminée
      (bind _structout (setmembers `/Game/Structure/S_Missions` :`StructRef` (`self.Array Element`) :`Etat` "NewEnumerator2"))
      (`KismetArrayLibrary.Array_Set` (`self.Missions`) (`self.Array Index`) _structout)
      ;[1 1 1] Mission suivante en cours
      (bind _result (`/Engine/EditorBlueprintResources/StandardMacros.IncrementInt` (`self.Array Index`))
        (:`  `
          (bind _output_get (set `local.NextIndex` _result))
          (if (< _output_get (`KismetArrayLibrary.Array_Length` (`self.Missions`)))
            (bind _structout_2 (setmembers `/Game/Structure/S_Missions` :`StructRef` (`|GetArrayItem` (`self.Missions`) (`local.NextIndex`)) :`Etat` "NewEnumerator1"))
            (`KismetArrayLibrary.Array_Set` (`self.Missions`) (`local.NextIndex`) _structout_2)
            (`self.AfficherMissionEncoursUI`)))))))

(fn `UserConstructionScript`)